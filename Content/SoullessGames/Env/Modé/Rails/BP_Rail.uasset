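; BP_Rail is a modular rail piece actor for environment building, whose mesh is chosen in the construction script.
; Its State switches the static mesh: Normal picks randomly from the AllRail array, Corner randomly from Corners, and Slope uses a fixed angled straight mesh.
; The event graph holds only disabled placeholder events, so there is no runtime logic.
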(fn `UserConstructionScript`
  (switch `/Game/SoullessGames/Proto/Core/Enum/E_RailState` (`self.State`)
    (:`NewEnumerator0`
      (`StaticMeshComponent.SetStaticMesh` (`self.StaticMesh`) (`KismetArrayLibrary.Array_Random` (`self.AllRail`))))
    (:`NewEnumerator1`
      (`StaticMeshComponent.SetStaticMesh` (`self.StaticMesh`) (`KismetArrayLibrary.Array_Random` (`self.Corners`))))
    (:`NewEnumerator2`
      (`StaticMeshComponent.SetStaticMesh` (`self.StaticMesh`) "/Game/SoullessGames/Env/Modé/Rails/SM_Rail-StraightAngle_128x128x16_.SM_Rail-StraightAngle_128x128x16_"))))