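; BP_Baleine is an environment actor, a whale by its name, that loops along a spline.
; If Activated is false, BeginPlay waits DelayToStart, then enables movement and starts a looping sound timer, whose random interval is rolled once.
; Each Tick advances Alpha by Speed over spline length, unscaled by delta time, places the Scene component at that point and rotation, and wraps at the end.
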(event `self.ReceiveBeginPlay`
  (if (not (`self.activated?`))
    (`KismetSystemLibrary.Delay` (`self.DelayToStart`))
    (set `self.canMove` true)
    (`KismetSystemLibrary.K2_SetTimerDelegate` (delegate `sound`) (`KismetMathLibrary.RandomFloatInRange` 10.0 40.0) true)))

(event `sound`
  (`AudioComponent.Play` (`self.Audio`) 0.0))

(event `self.ReceiveTick`
  (params (DeltaSeconds :type "Float (single-precision)"))
  (bind _spline (`self.Spline`))
  (bind _returnvalue (`KismetMathLibrary.Lerp` 0.0 (`SplineComponent.GetSplineLength` _spline) (`self.Alpha`)))
  (bind (_returnvalue_roll _returnvalue_pitch _returnvalue_yaw) (`KismetMathLibrary.BreakRotator` (`SplineComponent.GetRotationAtDistanceAlongSpline` _spline _returnvalue "Local")))
  (if (`self.canMove`)
    (set `self.Alpha` (+ (`KismetMathLibrary.NormalizeToRange` (`self.Speed`) 0.0 (`SplineComponent.GetSplineLength` (`self.Spline`))) (`self.Alpha`)))
    (`SceneComponent.K2_SetRelativeLocationAndRotation` (`self.Scene`) (`SplineComponent.GetLocationAtDistanceAlongSpline` _spline _returnvalue "Local") (`KismetMathLibrary.MakeRotator` _returnvalue_roll _returnvalue_pitch _returnvalue_yaw) false false)
    (if (>= (`self.Alpha`) 1.0)
      (set `self.Alpha` 0.0))))

(fn `UserConstructionScript`)