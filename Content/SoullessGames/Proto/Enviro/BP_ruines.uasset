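; BP_ruines is an environment ruins actor that hides 1000 units below its placed position at BeginPlay and moves when activated.
; Activated fires once, storing the lowered location and playing a timeline that adds a Z offset to it with a swept move, presumably raising the ruins.
; In parallel, a delayed 2D sound plays briefly and then fades out.
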(event `self.ReceiveBeginPlay`
  (bind (_returnvalue_x _returnvalue_y _returnvalue_z) (`KismetMathLibrary.BreakVector` (`self.K2_GetActorLocation`)))
  (`self.K2_SetActorLocation` (`KismetMathLibrary.MakeVector` _returnvalue_x _returnvalue_y (- _returnvalue_z 1000.0)) false true))

(event `Activated`
  (bind (_newvar_0_x _newvar_0_y _newvar_0_z) (`KismetMathLibrary.BreakVector` (`self.NewVar_0`)))
  (`/Engine/EditorBlueprintResources/StandardMacros.DoOnce` false
    (:`Completed`
      (set `self.NewVar_0` (`self.K2_GetActorLocation`))
      (`|ExecutionSequence`
        (:`then_0`
          (bind (_direction _newtrack_0) (`Timeline|Timeline_0` :!via `PlayFromStart`)
            (:`Update`
              (`self.K2_SetActorLocation` (`KismetMathLibrary.MakeVector` _newvar_0_x _newvar_0_y (+ _newvar_0_z _newtrack_0)) true))))
        (:`then_1`
          (`KismetSystemLibrary.Delay` 1.75)
          (bind _returnvalue (`GameplayStatics.CreateSound2D` "/Game/SoullessGames/Music/622798__e0fd96__2022-01-01-lingjiushan-bell-okm-ii-003__1_.622798__e0fd96__2022-01-01-lingjiushan-bell-okm-ii-003__1_" 1.0 1.0 0.0 null))
          (`AudioComponent.Play` _returnvalue 0.0)
          (`KismetSystemLibrary.Delay` 1.5)
          (`AudioComponent.FadeOut` _returnvalue 0.5 0.0 "Linear"))))))

(fn `UserConstructionScript`)