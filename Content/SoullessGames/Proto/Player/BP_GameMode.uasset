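; BP_GameMode is the game mode that creates the main HUD widget and handles save and reload-last-save.
; On BeginPlay it binds handlers to the save and reload events and adds WBP_Main to the viewport.
; Saving stores only a respawn transform in LastTP.
; Reload destroys the current character, spawns a new BP_Character at LastTP and calls Reset on every BP_ObjetParent actor.
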(event `self.ReceiveBeginPlay`
  (add `self.Save` (delegate `SaveEvent`))
  (add `self.ReloadLastSave` (delegate `reload`))
  (bind _returnvalue (`|CreateWidget` "/Game/SoullessGames/Proto/UI/WBP_Main.WBP_Main_C"))
  (`UserWidget.AddToViewport` _returnvalue 0))

(event `SaveEvent` :!signature `self.Save`
  (params (Pos :type "Vector Structure"))
  (set `self.LastTP` Pos))

(event `reload`
  (`self.K2_DestroyActor` (`/Game/SoullessGames/Proto/Core/BP_Library.GetChara`))
  (`|SpawnActorFromClass` "/Game/SoullessGames/Proto/Player/BP_Character.BP_Character_C" (`KismetMathLibrary.MakeTransform` (`self.LastTP`)) "Undefined" "OverrideRootScale" null null)
  (bind _outactors (`GameplayStatics.GetAllActorsOfClass` "/Game/SoullessGames/Proto/Blueprint/BP_ObjetParent.BP_ObjetParent_C"))
  (for _array_element _outactors
    (`/Game/SoullessGames/Proto/Blueprint/BP_ObjetParent.Reset` _array_element)))

(fn `UserConstructionScript`)