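; Player controller that shows the mouse cursor, lets the player click and drag world objects, and opens the pause menu.
; Click line-traces under the cursor to select a BP_ObjetParent, and release calls StopHold and clears the selection.
; While held, summed mouse X and Y movement is remapped through a curve, scaled by delta time, debug-printed and passed to EventHold.
; Pause input creates W_PauseMenu and pauses the game.
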(event `InputAction|PauseMenu`
  (params (Key :type "Key Structure"))
  (:`Pressed`
    (`|ExecutionSequence`
      (:`then_0`
        (bind _returnvalue (`|CreateWidget` "/Game/SoullessGames/Menu/W_PauseMenu.W_PauseMenu_C"))
        (bind _output_get (set `self.PauseMenu` _returnvalue))
        (`UserWidget.AddToViewport` _returnvalue 0)
        (`UserWidget.AddToViewport` _output_get 0))
      (:`then_1`
        (`GameplayStatics.SetGamePaused` true)))))

(event `self.ReceiveBeginPlay`
  (set `self.bShowMouseCursor` true))

(event `self.ReceiveTick`
  (params (DeltaSeconds :type "Float (single-precision)"))
  (`/Engine/EditorBlueprintResources/StandardMacros.IsValid` (`self.SelectedObject`)))

(event `InputAction|Clic`
  (params (Key :type "Key Structure"))
  (bind (_worldlocation _worlddirection) (`self.DeprojectMousePositionToWorld`))
  (bind _selectedobject (`self.SelectedObject`))
  (:`Pressed`
    (bind _outhit (`KismetSystemLibrary.LineTraceSingle` _worldlocation (+ _worldlocation (* _worlddirection 100000.0)) "TraceTypeQuery1"))
    (bind _asbp_objet_parent (cast `/Game/SoullessGames/Proto/Blueprint/BP_ObjetParent` (`.HitActor` (`GameplayStatics.BreakHitResult` _outhit))))
    (set `self.SelectedObject` _asbp_objet_parent))
  (:`Released`
    (`/Engine/EditorBlueprintResources/StandardMacros.IsValid` _selectedobject
      (:`Is Valid`
        (`/Game/SoullessGames/Proto/Blueprint/BP_ObjetParent.StopHold` _selectedobject)
        (set `self.SelectedObject` null)))))

(event `InputVectorAxis|Mouse2D`
  (params (AxisValue :type "Vector Structure"))
  (bind _returnvalue (* (`CurveFloat.GetFloatValue` (`self.Curve`) (`self.MoveToAdd`)) (`GameplayStatics.GetWorldDeltaSeconds`)))
  (`/Engine/EditorBlueprintResources/StandardMacros.IsValid` (`self.SelectedObject`)
    (:`Is Valid`
      (set `self.MoveToAdd` (+ AxisValue_X AxisValue_Y))
      (`KismetSystemLibrary.PrintString` (`KismetStringLibrary.Conv_DoubleToString` _returnvalue))
      (`/Game/SoullessGames/Proto/Blueprint/BP_ObjetParent.EventHold` (`self.SelectedObject`) _returnvalue))))

(fn `UserConstructionScript`)