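; Player character prototype that triggers a save whenever its Bille component slows below a speed threshold.
; Tick compares the Bille's velocity to VeloToSave and passes the game mode a position raised above the Bille to save.
; A DoOnce gate limits this to one save per slowdown and rearms once the speed is back at or above the threshold.
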(event `self.ReceiveBeginPlay`)

(event `self.ReceiveTick`
  (params (DeltaSeconds :type "Float (single-precision)"))
  (if (< (`KismetMathLibrary.VSize` (`SceneComponent.GetComponentVelocity` (`self.Bille`))) (`self.VeloToSave`))
    (`/Engine/EditorBlueprintResources/StandardMacros.DoOnce` true :!label _label
      (:`Completed`
        (`/Game/SoullessGames/Proto/Player/BP_GameMode.Save` (`/Game/SoullessGames/Proto/Core/BP_Library.GetMyGamemode`) (+ (`SceneComponent.K2_GetComponentLocation` (`self.Bille`)) (0.0 0.0 100.0)))
        (`KismetSystemLibrary.PrintString` "saveo")))
    (else
      (goto _label :!via `Reset`))))

(fn `UserConstructionScript`)