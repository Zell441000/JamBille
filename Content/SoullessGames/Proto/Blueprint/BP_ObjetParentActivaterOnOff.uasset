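; BP_ObjetParentActivaterOnOff is a prototype activator Blueprint that switches a set of linked objects on and off in response to hold events.
; EventHold loops over the Objects array and calls On on each entry, while StopHold calls Off on the same entries.
; It has no other active logic, as BeginPlay, overlap and Tick are disabled stubs and the construction script only calls its parent.
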(event `self.EventHold`
  (params (ValueToAdd :type "Float (double-precision)"))
  (for _array_element (`self.Objects`)
    (`/Game/SoullessGames/Proto/Blueprint/BP_ObjetParentOnOff.On` _array_element)))

(event `self.StopHold`
  (for _array_element (`self.Objects`)
    (`/Game/SoullessGames/Proto/Blueprint/BP_ObjetParentOnOff.Off` _array_element)))

(fn `UserConstructionScript`
  (`parent.UserConstructionScript`))