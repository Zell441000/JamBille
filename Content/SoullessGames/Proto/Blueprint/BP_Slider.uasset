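; BP_Slider is an actor that lays out a straight slide of evenly spaced segments along a given direction.
; SetNewSlide moves and rotates it to the origin, then adds local-space mesh instances along X, spawning a BP_SliderChild at each one's world location.
; EndSlide tracks the next segment's offset.
; Releasse calls Reset, which clears the instances, destroys every BP_SliderChild in the world and zeroes EndSlide inside that loop.
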(event `SetNewSlide`
  (params (originValue :type "Vector Structure") (direction :type "Vector Structure") (NumberLenght :type Integer))
  (bind _returnvalue (`KismetMathLibrary.Conv_VectorToRotator` direction))
  (`self.K2_SetActorRotation` _returnvalue)
  (`self.K2_SetActorLocation` originValue false true)
  (for _ (range 1 (+ NumberLenght 1))
    (bind _returnvalue_2 (`InstancedStaticMeshComponent.AddInstance` (`self.InstancedStaticMesh`) (`KismetMathLibrary.Conv_VectorToTransform` (`self.EndSlide`)) false))
    (`|SpawnActorFromClass` "/Game/SoullessGames/Proto/Blueprint/BP_SliderChild.BP_SliderChild_C" (`KismetMathLibrary.MakeTransform` (.location (`InstancedStaticMeshComponent.GetInstanceTransform` (`self.InstancedStaticMesh`) _returnvalue_2 true)) _returnvalue) "Undefined" "OverrideRootScale" null null)
    (set `self.EndSlide` (+ (`self.EndSlide`) (128.0 0.0 0.0)))))

(event `Releasse`
  (`self.Reset`))

(fn `Reset`
  (`InstancedStaticMeshComponent.ClearInstances` (`self.InstancedStaticMesh`))
  (bind _outactors (`GameplayStatics.GetAllActorsOfClass` "/Game/SoullessGames/Proto/Blueprint/BP_SliderChild.BP_SliderChild_C"))
  (for _array_element _outactors
    (`self.K2_DestroyActor` _array_element)
    (set `self.EndSlide` (0.0 0.0 0.0))))

(fn `UserConstructionScript`)