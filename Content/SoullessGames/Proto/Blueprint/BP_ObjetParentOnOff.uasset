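; Base actor, going by its name, for on/off objects that slide along a chosen world axis within limits set at BeginPlay.
; Each On call pauses the return timer and takes one swept step toward the maximum, a multiple of 128 units from the origin.
; Off starts a looping frame-delta timer that steps the actor back until it passes its starting value.
; Reverse movement for Y offsets X instead.
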(event `self.ReceiveBeginPlay`
  (`parent.ReceiveBeginPlay`)
  (`self.SetValeurMovement`))

(event `On`
  (`KismetSystemLibrary.K2_PauseTimerHandle` (stale `Off` _returnvalue))
  (bind _stop (`self.CheckFinish` false))
  (if (not _stop)
    (switch `/Game/SoullessGames/Proto/Core/Enum/E_MovementsDirection` (`self.MovementDirection`)
      (:`NewEnumerator0`
        (`self.K2_AddActorWorldOffset` (`KismetMathLibrary.MakeVector` 0.0 0.0 (`self.Speed`)) true))
      (:`NewEnumerator1`
        (`self.K2_AddActorWorldOffset` (`KismetMathLibrary.MakeVector` (`self.Speed`)) true))
      (:`NewEnumerator2`
        (`self.K2_AddActorWorldOffset` (`KismetMathLibrary.MakeVector` 0.0 (`self.Speed`)) true)))))

(event `Off`
  (bind _returnvalue (`KismetSystemLibrary.K2_SetTimerDelegate` (delegate `ReverseMove`) (`GameplayStatics.GetWorldDeltaSeconds`) true)))

(event `ReverseMove`
  (bind _stop (`self.CheckFinish` true))
  (if (not _stop)
    (switch `/Game/SoullessGames/Proto/Core/Enum/E_MovementsDirection` (`self.MovementDirection`)
      (:`NewEnumerator0`
        (`self.K2_AddActorWorldOffset` (`KismetMathLibrary.MakeVector` 0.0 0.0 (* (`self.Speed`) -1.0)) true))
      (:`NewEnumerator1`
        (`self.K2_AddActorWorldOffset` (`KismetMathLibrary.MakeVector` (* (`self.Speed`) -1.0)) true))
      (:`NewEnumerator2`
        (`self.K2_AddActorWorldOffset` (`KismetMathLibrary.MakeVector` (* (`self.Speed`) -1.0)) true)))
    (else
      (`KismetSystemLibrary.K2_PauseTimerHandle` (stale `Off` _returnvalue)))))

(fn `CheckFinish`
  (params (`Reverse?` :type Boolean))
  (returns (stop :type Boolean))
  (bind (_returnvalue_x _returnvalue_y _returnvalue_z) (`KismetMathLibrary.BreakVector` (`self.K2_GetActorLocation`)))
  (bind _returnvalue (select `/Game/SoullessGames/Proto/Core/Enum/E_MovementsDirection` (`self.MovementDirection`) :`NewEnumerator0` _returnvalue_z :`NewEnumerator1` _returnvalue_x :`NewEnumerator2` _returnvalue_y))
  (if `Reverse?`
    (if (< _returnvalue (`self.ValeurMin`))
      _
      (else
        (return false)))
    (elif (> _returnvalue (`self.ValeurMax`))
      _
      (else
        (return false))))
  (return true))

(fn `SetValeurMovement`
  (bind (_originlocation_x _originlocation_y _originlocation_z) (`KismetMathLibrary.BreakVector` (`self.OriginLocation`)))
  (set `self.OriginLocation` (`self.K2_GetActorLocation`))
  (set `self.ValeurMin` (select `/Game/SoullessGames/Proto/Core/Enum/E_MovementsDirection` (`self.MovementDirection`) :`NewEnumerator0` _originlocation_z :`NewEnumerator1` _originlocation_x :`NewEnumerator2` _originlocation_y))
  (set `self.ValeurMax` (+ (`self.ValeurMin`) (* 128.0 (`self.Movementpossible`)))))

(fn `UserConstructionScript`
  (`parent.UserConstructionScript`))