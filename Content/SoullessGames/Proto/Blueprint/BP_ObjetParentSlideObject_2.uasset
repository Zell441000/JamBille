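; Parent Blueprint for objects that slide along one world axis, chosen by MovementDirection.
; On BeginPlay it stores the origin and derives min and max bounds from MovementPosible in 128-unit steps.
; EventHold applies a swept world offset only while CheckSlide finds the current position within the bound in that direction, so a move can overshoot.
; Reset teleports the object back to its origin.
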(event `self.ReceiveBeginPlay`
  (`parent.ReceiveBeginPlay`)
  (`self.SetValeurMovement`))

(event `self.Reset`
  (`self.K2_SetActorLocation` (`self.OriginLocation`) false true))

(event `self.EventHold`
  (params (ValueToAdd :type "Float (double-precision)"))
  (bind _returnvalue (`self.CheckSlide` ValueToAdd))
  (if _returnvalue
    (switch `/Game/SoullessGames/Proto/Core/Enum/E_MovementsDirection` (`self.MovementDirection`)
      (:`NewEnumerator0`
        (`self.K2_AddActorWorldOffset` (`KismetMathLibrary.MakeVector` 0.0 0.0 ValueToAdd) true))
      (:`NewEnumerator1`
        (`self.K2_AddActorWorldOffset` (`KismetMathLibrary.MakeVector` ValueToAdd) true))
      (:`NewEnumerator2`
        (`self.K2_AddActorWorldOffset` (`KismetMathLibrary.MakeVector` 0.0 ValueToAdd) true)))))

(fn `CheckSlide`
  (params (ValueToAdd :type "Float (double-precision)"))
  (returns (ReturnValue :type Boolean))
  (bind (_returnvalue_x _returnvalue_y _returnvalue_z) (`KismetMathLibrary.BreakVector` (`self.K2_GetActorLocation`)))
  (bind _returnvalue (select `/Game/SoullessGames/Proto/Core/Enum/E_MovementsDirection` (`self.MovementDirection`) :`NewEnumerator0` _returnvalue_z :`NewEnumerator1` _returnvalue_x :`NewEnumerator2` _returnvalue_y))
  (if (< ValueToAdd 0.0)
    (if (not (< _returnvalue (`self.ValeurMin`)))
      _
      (else
        (return false)))
    (elif (not (> _returnvalue (`self.ValeurMax`)))
      _
      (else
        (return false))))
  (return true))

(fn `SetValeurMovement`
  (locals (Valor1 :type "Float (double-precision)") (Valor2 :type "Float (double-precision)"))
  (bind (_originlocation_x _originlocation_y _originlocation_z) (`KismetMathLibrary.BreakVector` (`self.OriginLocation`)))
  (set `self.OriginLocation` (`self.K2_GetActorLocation`))
  (set `local.Valor1` (select `/Game/SoullessGames/Proto/Core/Enum/E_MovementsDirection` (`self.MovementDirection`) :`NewEnumerator0` _originlocation_z :`NewEnumerator1` _originlocation_x :`NewEnumerator2` _originlocation_y))
  (set `local.Valor2` (+ (`local.Valor1`) (* 128.0 (`self.MovementPosible`))))
  (set `self.ValeurMax` (`KismetMathLibrary.FMax` (`local.Valor1`) (`local.Valor2`)))
  (set `self.ValeurMin` (`KismetMathLibrary.FMin` (`local.Valor1`) (`local.Valor2`))))

(fn `UserConstructionScript`
  (`parent.UserConstructionScript`))