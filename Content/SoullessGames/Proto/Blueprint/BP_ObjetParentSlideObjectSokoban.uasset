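; Sokoban-style sliding puzzle object that held input moves along one axis between its start position and a MovementMax-scaled end.
; EventHold accumulates scaled, optionally negated input into a clamped alpha, which lerps the swept actor position.
; Tick line-traces toward the input direction, with debug drawing and printing, clearing CanMove when another such object is hit.
; Reset restores the origin; CheckSlide tests the slide bounds but is not called here.
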(event `self.ReceiveTick`
  (params (DeltaSeconds :type "Float (single-precision)"))
  (bind _vector (`self.Vector`))
  (bind _returnvalue (`SceneComponent.K2_GetComponentLocation` (`self.Forward`)))
  (bind _returnvalue_2 (`SceneComponent.K2_GetComponentLocation` (`self.Right`)))
  (bind _returnvalue_3 (`SceneComponent.K2_GetComponentLocation` (`self.BAckWard`)))
  (bind _returnvalue_4 (`SceneComponent.K2_GetComponentLocation` (`self.Left`)))
  (bind _returnvalue_5 (> (`self.Value to Add`) 0.0))
  (`KismetSystemLibrary.PrintString` (`KismetStringLibrary.Conv_DoubleToString` (`self.Value to Add`)))
  (bind (_outhit _returnvalue_6) (`KismetSystemLibrary.LineTraceSingle` (select `/Game/SoullessGames/Proto/Core/Enum/E_VectorType` _vector :`NewEnumerator0` (`KismetMathLibrary.SelectVector` _returnvalue _returnvalue_3 _returnvalue_5) :`NewEnumerator1` (`KismetMathLibrary.SelectVector` _returnvalue_2 _returnvalue_4 _returnvalue_5)) (select `/Game/SoullessGames/Proto/Core/Enum/E_VectorType` _vector :`NewEnumerator0` (`KismetMathLibrary.SelectVector` (+ _returnvalue (* (`self.GetActorForwardVector`) (`self.lenght`))) (+ _returnvalue_3 (* (* (`self.GetActorForwardVector`) -1.0) (`self.lenght`))) _returnvalue_5) :`NewEnumerator1` (`KismetMathLibrary.SelectVector` (+ _returnvalue_2 (* (`self.GetActorRightVector`) (`self.lenght`))) (+ _returnvalue_4 (* (* (`self.GetActorRightVector`) -1.0) (`self.lenght`))) _returnvalue_5)) "TraceTypeQuery1" false (`|MakeArray` self :!type "Actor Object Reference") "ForDuration" true (struct :`R` 1.0 :`A` 1.0) (struct :`G` 1.0 :`A` 1.0) 0.5))
  (if _returnvalue_6
    (cast `/Game/SoullessGames/Proto/Blueprint/BP_ObjetParentSlideObjectSokoban` (`.HitActor` (`GameplayStatics.BreakHitResult` _outhit)))
    (set `self.CanMove` false)
    (else
      (set `self.CanMove` true))))

(event `self.ReceiveBeginPlay`
  (`parent.ReceiveBeginPlay`)
  (`self.SetValeurMovement`))

(event `self.Reset`
  (`self.K2_SetActorLocation` (`self.OriginLocation`) false true)
  (set `self.TotalMoveInput` 0.0))

(event `self.EventHold`
  (params (ValueToAdd :type "Float (double-precision)"))
  (bind (_originlocation_x _originlocation_y _originlocation_z) (`KismetMathLibrary.BreakVector` (`self.OriginLocation`)))
  (bind _returnvalue (* ValueToAdd (`self.Sensi`)))
  (if (== ValueToAdd 0.0)
    (set `self.Hold` false)
    (else
      (set `self.Value to Add` ValueToAdd)
      (set `self.Hold` true)))
  (if (`self.CanMove`)
    (bind _output_get (set `self.TotalMoveInput` (`KismetMathLibrary.FClamp` (+ (select `bool` (`self.Negate`) :`false` _returnvalue :`true` (* _returnvalue -1.0)) (`self.TotalMoveInput`)))))
    (switch `/Game/SoullessGames/Proto/Core/Enum/E_MovementsDirection` (`self.MovementDirection`)
      (:`NewEnumerator1`
        (bind _returnvalue_2 (`KismetMathLibrary.Lerp` (`self.ValeurOrign`) (`self.ValorEndSlide`) _output_get))
        (`self.K2_SetActorLocation` (`KismetMathLibrary.MakeVector` _returnvalue_2 _originlocation_y _originlocation_z) true))
      (:`NewEnumerator2`
        (`self.K2_SetActorLocation` (`KismetMathLibrary.MakeVector` _originlocation_x _returnvalue_2 _originlocation_z) true))
      (:`NewEnumerator0`
        (`self.K2_SetActorLocation` (`KismetMathLibrary.MakeVector` _originlocation_x _originlocation_y _returnvalue_2) true)))))

(fn `CheckSlide`
  (params (ValueToAdd :type "Float (double-precision)"))
  (returns (ReturnValue :type Boolean))
  (bind (_returnvalue_x _returnvalue_y _returnvalue_z) (`KismetMathLibrary.BreakVector` (`self.K2_GetActorLocation`)))
  (bind _returnvalue (select `/Game/SoullessGames/Proto/Core/Enum/E_MovementsDirection` (`self.MovementDirection`) :`NewEnumerator1` _returnvalue_x :`NewEnumerator2` _returnvalue_y :`NewEnumerator0` _returnvalue_z))
  (if (< ValueToAdd 0.0)
    (if (not (< _returnvalue (`self.ValeurOrign`)))
      _
      (else
        (return false)))
    (elif (not (> _returnvalue (`self.ValorEndSlide`)))
      _
      (else
        (return false))))
  (return true))

(fn `SetValeurMovement`
  (bind (_originlocation_x _originlocation_y _originlocation_z) (`KismetMathLibrary.BreakVector` (`self.OriginLocation`)))
  (set `self.OriginLocation` (`self.K2_GetActorLocation`))
  (set `self.ValeurOrign` (select `/Game/SoullessGames/Proto/Core/Enum/E_MovementsDirection` (`self.MovementDirection`) :`NewEnumerator1` _originlocation_x :`NewEnumerator2` _originlocation_y :`NewEnumerator0` _originlocation_z))
  (set `self.ValorEndSlide` (+ (`self.ValeurOrign`) (* 128.0 (`self.MovementMax`)))))

(fn `UserConstructionScript`
  (`parent.UserConstructionScript`)
  (if (`self.Verti`)
    (`SceneComponent.SetVisibility` (`self.Cube7`) true true)))