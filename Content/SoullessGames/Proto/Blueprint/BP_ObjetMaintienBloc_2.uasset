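; Hold-to-move block that slides along a chosen X, Y or Z axis while held and creeps back after release.
; BeginPlay derives travel limits from the start position and a count of 128-unit steps.
; EventHold applies swept offsets for non-negative input inside those limits, with Negate flipping X and Y.
; StopHold starts a looping frame-interval timer that steps the block back, pausing once it passes the start value.
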(event `self.ReceiveBeginPlay`
  (`parent.ReceiveBeginPlay`)
  (`self.SetValeurMovement`))

(event `self.Reset`)

(event `self.EventHold`
  (params (ValueToAdd :type "Float (double-precision)"))
  (bind _returnvalue (`self.CheckSlide` ValueToAdd))
  (if _returnvalue
    (switch `/Game/SoullessGames/Proto/Core/Enum/E_MovementsDirection` (`self.Movement Direction`)
      (:`NewEnumerator0`
        (`SceneComponent.K2_AddRelativeLocation` (`self.DefaultSceneRoot`) (`KismetMathLibrary.MakeVector` 0.0 0.0 ValueToAdd) true false))
      (:`NewEnumerator1`
        (`SceneComponent.K2_AddRelativeLocation` (`self.DefaultSceneRoot`) (`KismetMathLibrary.MakeVector` (select `bool` (`self.Negate`) :`false` ValueToAdd :`true` (* ValueToAdd -1.0))) true false))
      (:`NewEnumerator2`
        (`SceneComponent.K2_AddRelativeLocation` (`self.DefaultSceneRoot`) (`KismetMathLibrary.MakeVector` 0.0 (select `bool` (`self.Negate`) :`false` ValueToAdd :`true` (* ValueToAdd -1.0))) true false)))))

(event `self.StopHold`
  (bind _returnvalue (`KismetSystemLibrary.K2_SetTimerDelegate` (delegate `ReverseMove`) (`GameplayStatics.GetWorldDeltaSeconds`) true)))

(event `ReverseMove`
  (if (`self.Negate`)
    (bind _stop (`self.CheckFinish_0` false))
    (if (not _stop)
      (switch `/Game/SoullessGames/Proto/Core/Enum/E_MovementsDirection` (`self.Movement Direction`) :!label _label
        (:`NewEnumerator0`
          (`SceneComponent.K2_AddRelativeLocation` (`self.DefaultSceneRoot`) (`KismetMathLibrary.MakeVector` 0.0 0.0 (select `bool` (`self.Negate`) :`false` -5.0 :`true` 5.0)) true false))
        (:`NewEnumerator1`
          (`SceneComponent.K2_AddRelativeLocation` (`self.DefaultSceneRoot`) (`KismetMathLibrary.MakeVector` (select `bool` (`self.Negate`) :`false` -5.0 :`true` 5.0)) true false))
        (:`NewEnumerator2`
          (`SceneComponent.K2_AddRelativeLocation` (`self.DefaultSceneRoot`) (`KismetMathLibrary.MakeVector` 0.0 (select `bool` (`self.Negate`) :`false` -5.0 :`true` 5.0)) true false)))
      (else
        (`KismetSystemLibrary.K2_PauseTimerHandle` (stale `self.StopHold` _returnvalue) :!label _label_2)))
    (else
      (bind _stop_2 (`self.CheckFinish` false))
      (if (not _stop_2)
        (goto _label)
        (else
          (goto _label_2))))))

(fn `CheckFinish`
  (params (`Reverse?` :type Boolean))
  (returns (stop :type Boolean))
  (bind (_relativelocation_x _relativelocation_y _relativelocation_z) (`KismetMathLibrary.BreakVector` (`SceneComponent.RelativeLocation` (`self.DefaultSceneRoot`))))
  (if (< (select `/Game/SoullessGames/Proto/Core/Enum/E_MovementsDirection` (`self.Movement Direction`) :`NewEnumerator0` _relativelocation_z :`NewEnumerator1` _relativelocation_x :`NewEnumerator2` _relativelocation_y) (`self.Valeur Min`))
    (return true)
    (else
      (return false))))

(fn `CheckFinish_0`
  (params (`Reverse?` :type Boolean))
  (returns (stop :type Boolean))
  (bind (_relativelocation_x _relativelocation_y _relativelocation_z) (`KismetMathLibrary.BreakVector` (`SceneComponent.RelativeLocation` (`self.DefaultSceneRoot`))))
  (if (> (select `/Game/SoullessGames/Proto/Core/Enum/E_MovementsDirection` (`self.Movement Direction`) :`NewEnumerator0` _relativelocation_z :`NewEnumerator1` _relativelocation_x :`NewEnumerator2` _relativelocation_y) (`self.Valeur Min`))
    (return true)
    (else
      (return false))))

(fn `CheckSlide`
  (params (ValueToAdd :type "Float (double-precision)"))
  (returns (ReturnValue :type Boolean))
  (bind (_returnvalue_x _returnvalue_y _returnvalue_z) (`KismetMathLibrary.BreakVector` (`self.K2_GetActorLocation`)))
  (bind _returnvalue (select `/Game/SoullessGames/Proto/Core/Enum/E_MovementsDirection` (`self.Movement Direction`) :`NewEnumerator0` _returnvalue_z :`NewEnumerator1` _returnvalue_x :`NewEnumerator2` _returnvalue_y))
  (if (< ValueToAdd 0.0)
    _
    (elif (and (< _returnvalue (`self.ValeurMax`)) (> _returnvalue (`self.Valeur Min`)))
      (return true)
      (else
        _)))
  (return false))

(fn `SetValeurMovement`
  (bind (_relativelocation_x _relativelocation_y _relativelocation_z) (`KismetMathLibrary.BreakVector` (`SceneComponent.RelativeLocation` (`self.DefaultSceneRoot`))))
  (set `self.Valeur Min` (select `/Game/SoullessGames/Proto/Core/Enum/E_MovementsDirection` (`self.Movement Direction`) :`NewEnumerator0` _relativelocation_z :`NewEnumerator1` _relativelocation_x :`NewEnumerator2` _relativelocation_y))
  (set `self.ValeurMax` (+ (`self.Valeur Min`) (* 128.0 (`self.MovementPosible`)))))

(fn `UserConstructionScript`
  (`parent.UserConstructionScript`))