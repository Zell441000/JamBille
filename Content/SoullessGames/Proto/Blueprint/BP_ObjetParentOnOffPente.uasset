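; Switchable slope (pente) object that tilts its static mesh between two roll angles when turned on or off.
; BeginPlay sets the roll to ValeurMin, then On and Off each play their own timeline to lerp it toward ValeurMax or back, with sweep.
; Off also stops the On timeline, but On leaves the Off timeline running.
; CheckFinish and SetValeurMovement handle axis-based location limits but are not called in these graphs.
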(event `self.ReceiveBeginPlay`
  (bind (_relativerotation_roll _relativerotation_pitch _relativerotation_yaw) (`KismetMathLibrary.BreakRotator` (`SceneComponent.RelativeRotation` (`self.StaticMesh`))))
  (`parent.ReceiveBeginPlay`)
  (`SceneComponent.K2_SetRelativeRotation` (`self.StaticMesh`) (`KismetMathLibrary.MakeRotator` (`self.ValeurMin`) _relativerotation_pitch _relativerotation_yaw) true false))

(event `self.On`
  (bind (_relativerotation_roll _relativerotation_pitch _relativerotation_yaw) (`KismetMathLibrary.BreakRotator` (`SceneComponent.RelativeRotation` (`self.StaticMesh`))))
  (bind (_direction _newtrack_0) (`Timeline|Timeline_0` :!via `PlayFromStart` :!label _label)
    (:`Update`
      (`SceneComponent.K2_SetRelativeRotation` (`self.StaticMesh`) (`KismetMathLibrary.MakeRotator` (`KismetMathLibrary.Lerp` (`self.ValeurMin`) (`self.ValeurMax`) _newtrack_0) _relativerotation_pitch _relativerotation_yaw) true false))))

(event `self.Off`
  (bind (_relativerotation_roll _relativerotation_pitch _relativerotation_yaw) (`KismetMathLibrary.BreakRotator` (`SceneComponent.RelativeRotation` (`self.StaticMesh`))))
  (`|ExecutionSequence`
    (:`then_0`
      (bind (_direction _newtrack_0) (`Timeline|Timeline_1` :!via `PlayFromStart`)
        (:`Update`
          (`SceneComponent.K2_SetRelativeRotation` (`self.StaticMesh`) (`KismetMathLibrary.MakeRotator` (`KismetMathLibrary.Lerp` (`self.ValeurMax`) (`self.ValeurMin`) _newtrack_0) _relativerotation_pitch _relativerotation_yaw) true false))))
    (:`then_1`
      (goto _label :!via `Stop`))))

(fn `CheckFinish`
  (params (`Reverse?` :type Boolean))
  (returns (stop :type Boolean))
  (bind (_returnvalue_x _returnvalue_y _returnvalue_z) (`KismetMathLibrary.BreakVector` (`self.K2_GetActorLocation`)))
  (bind _returnvalue (select `/Game/SoullessGames/Proto/Core/Enum/E_MovementsDirection` (`self.MovementDirection`) :`NewEnumerator1` _returnvalue_x :`NewEnumerator2` _returnvalue_y :`NewEnumerator0` _returnvalue_z))
  (if `Reverse?`
    (if (< _returnvalue (`self.ValeurMin`))
      _
      (else
        (return false)))
    (elif (> _returnvalue (`self.ValeurMax`))
      _
      (else
        (return false))))
  (return true))

(fn `SetValeurMovement`
  (bind (_originlocation_x _originlocation_y _originlocation_z) (`KismetMathLibrary.BreakVector` (`self.OriginLocation`)))
  (set `self.OriginLocation` (`self.K2_GetActorLocation`))
  (set `self.ValeurMin` (select `/Game/SoullessGames/Proto/Core/Enum/E_MovementsDirection` (`self.MovementDirection`) :`NewEnumerator1` _originlocation_x :`NewEnumerator2` _originlocation_y :`NewEnumerator0` _originlocation_z))
  (set `self.ValeurMax` (+ (`self.ValeurMin`) (* 128.0 (`self.Movementpossible`)))))

(fn `UserConstructionScript`
  (`parent.UserConstructionScript`))