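; BP_Ascenseur is a one-way elevator that rises when a BP_Character overlaps its Box trigger.
; The overlap turns on collision for four Cube walls and records the current height, then plays the Assenceur timeline from the start.
; The timeline lerps the actor upward with sweep by UnitToUp times 128 units, and the walls lose collision again when it finishes.
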(event `self.ReceiveBeginPlay`
  (`PrimitiveComponent.SetCollisionEnabled` (`self.Cube`) "NoCollision")
  (`PrimitiveComponent.SetCollisionEnabled` (`self.Cube2`) "NoCollision")
  (`PrimitiveComponent.SetCollisionEnabled` (`self.Cube1`) "NoCollision")
  (`PrimitiveComponent.SetCollisionEnabled` (`self.Cube3`) "NoCollision"))

(event `self.ReceiveActorBeginOverlap`
  (params (OtherActor :type "Actor Object Reference")))

(event `self.Box.OnComponentBeginOverlap`
  (params (OverlappedComponent :type "PrimitiveComponent Object Reference") (OtherActor :type "Actor Object Reference") (OtherComp :type "PrimitiveComponent Object Reference") (OtherBodyIndex :type Integer) (bFromSweep :type Boolean) (SweepResult :type "HitResult Structure (by ref)"))
  (bind (_returnvalue_x _returnvalue_y _returnvalue_z) (`KismetMathLibrary.BreakVector` (`self.K2_GetActorLocation`)))
  (bind (_returnvalue_x_2 _returnvalue_y_2) (`KismetMathLibrary.BreakVector` (`self.K2_GetActorLocation`)))
  (bind _return_value_z (`self.Return Value Z`))
  (cast `/Game/SoullessGames/Proto/Player/BP_Character` OtherActor)
  (`PrimitiveComponent.SetCollisionEnabled` (`self.Cube`) "QueryAndPhysics")
  (`PrimitiveComponent.SetCollisionEnabled` (`self.Cube2`) "QueryAndPhysics")
  (`PrimitiveComponent.SetCollisionEnabled` (`self.Cube1`) "QueryAndPhysics")
  (`PrimitiveComponent.SetCollisionEnabled` (`self.Cube3`) "QueryAndPhysics")
  (set `self.Return Value Z` _returnvalue_z)
  (bind (_direction _newtrack_0) (`Timeline|Assenceur` :!via `PlayFromStart`)
    (:`Update`
      (`self.K2_SetActorLocation` (`KismetMathLibrary.MakeVector` _returnvalue_x_2 _returnvalue_y_2 (`KismetMathLibrary.Lerp` _return_value_z (+ _return_value_z (* 128.0 (`self.UnitToUp`))) _newtrack_0)) true))
    (:`Finished`
      (`PrimitiveComponent.SetCollisionEnabled` (`self.Cube`) "NoCollision")
      (`PrimitiveComponent.SetCollisionEnabled` (`self.Cube2`) "NoCollision")
      (`PrimitiveComponent.SetCollisionEnabled` (`self.Cube1`) "NoCollision")
      (`PrimitiveComponent.SetCollisionEnabled` (`self.Cube3`) "NoCollision"))))

(fn `UserConstructionScript`)