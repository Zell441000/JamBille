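; Interactive slope prototype that pitches while held and returns to its starting pitch when released.
; Hold input accumulates into a clamped, sensitivity-scaled alpha, whose lerped value is added as local pitch, only for positive input below the maximum.
; Releasing starts a looping timer at frame-delta interval that rotates by Speed until pitch reaches the BeginPlay-recorded minimum, then pauses and snaps to it.
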(event `self.ReceiveBeginPlay`
  (`parent.ReceiveBeginPlay`)
  (`self.SetValeurMovement`))

(event `self.Reset`)

(event `self.EventHold`
  (params (ValueToAdd :type "Float (double-precision)"))
  (if (not (== ValueToAdd 0.0))
    (set `self.TotalTKT` (`KismetMathLibrary.FClamp` (+ (* ValueToAdd (`self.Sensi`)) (`self.TotalTKT`))))
    (bind _returnvalue (`self.CheckSlide` ValueToAdd))
    (if _returnvalue
      (`self.K2_AddActorLocalRotation` (`KismetMathLibrary.MakeRotator` 0.0 (`KismetMathLibrary.Lerp` (`self.Valeur Min`) (`self.ValeurMax`) (`self.TotalTKT`))) true true))))

(event `self.StopHold`
  (bind _returnvalue (`KismetSystemLibrary.K2_SetTimerDelegate` (delegate `ReverseMove`) (`GameplayStatics.GetWorldDeltaSeconds`) true)))

(event `ReverseMove`
  (bind (_returnvalue_roll _returnvalue_pitch _returnvalue_yaw) (`KismetMathLibrary.BreakRotator` (`self.K2_GetActorRotation`)))
  (bind _stop (`self.CheckFinish` true))
  (if (not _stop)
    (`self.K2_AddActorLocalRotation` (`KismetMathLibrary.MakeRotator` 0.0 (`self.Speed`)) true)
    (else
      (`KismetSystemLibrary.K2_PauseTimerHandle` (stale `self.StopHold` _returnvalue))
      (`self.K2_SetActorRotation` (`KismetMathLibrary.MakeRotator` _returnvalue_roll (`self.Valeur Min`) _returnvalue_yaw) true))))

(fn `CheckFinish`
  (params (`Reverse?` :type Boolean))
  (returns (stop :type Boolean))
  (bind (_returnvalue_roll _returnvalue_pitch) (`KismetMathLibrary.BreakRotator` (`self.K2_GetActorRotation`)))
  (if (> _returnvalue_pitch (`self.Valeur Min`))
    (return false)
    (else
      (return true))))

(fn `CheckSlide`
  (params (ValueToAdd :type "Float (double-precision)"))
  (returns (ReturnValue :type Boolean))
  (bind (_returnvalue_roll _returnvalue_pitch) (`KismetMathLibrary.BreakRotator` (`self.K2_GetActorRotation`)))
  (if (< ValueToAdd 0.0)
    _
    (elif (< _returnvalue_pitch (`self.ValeurMax`))
      (return true)
      (else
        _)))
  (return false))

(fn `SetValeurMovement`
  (bind (_returnvalue_roll _returnvalue_pitch) (`KismetMathLibrary.BreakRotator` (`self.K2_GetActorRotation`)))
  (set `self.Valeur Min` _returnvalue_pitch))

(fn `UserConstructionScript`
  (`parent.UserConstructionScript`))