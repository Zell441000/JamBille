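; Prototype block actor that slides along a chosen X, Y or Z axis while held and moves back on release.
; Hold events offset it by half the input, allowing only non-negative input below a maximum derived from MovementPosible.
; StopHold starts a looping timer at frame-delta intervals that applies Speed until the position drops below the minimum, then pauses.
; BeginPlay takes that minimum from the actor's rotation pitch, not its location.
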(event `self.ReceiveBeginPlay`
  (`parent.ReceiveBeginPlay`)
  (`self.SetValeurMovement`))

(event `self.Reset`)

(event `self.EventHold`
  (params (ValueToAdd :type "Float (double-precision)"))
  (bind _returnvalue (`self.CheckSlide` ValueToAdd))
  (if _returnvalue
    (switch `/Game/SoullessGames/Proto/Core/Enum/E_MovementsDirection` (`self.Movement Direction`)
      (:`NewEnumerator0`
        (`self.K2_AddActorWorldOffset` (`KismetMathLibrary.MakeVector` 0.0 0.0 (/ ValueToAdd 2.0))))
      (:`NewEnumerator1`
        (`self.K2_AddActorWorldOffset` (`KismetMathLibrary.MakeVector` (/ ValueToAdd 2.0))))
      (:`NewEnumerator2`
        (`self.K2_AddActorWorldOffset` (`KismetMathLibrary.MakeVector` 0.0 (/ ValueToAdd 2.0)))))))

(event `self.StopHold`
  (bind _returnvalue (`KismetSystemLibrary.K2_SetTimerDelegate` (delegate `ReverseMove`) (`GameplayStatics.GetWorldDeltaSeconds`) true)))

(event `ReverseMove`
  (bind _stop (`self.CheckFinish` true))
  (if (not _stop)
    (switch `/Game/SoullessGames/Proto/Core/Enum/E_MovementsDirection` (`self.Movement Direction`)
      (:`NewEnumerator0`
        (`self.K2_AddActorWorldOffset` (`KismetMathLibrary.MakeVector` 0.0 0.0 (`self.Speed`))))
      (:`NewEnumerator1`
        (`self.K2_AddActorWorldOffset` (`KismetMathLibrary.MakeVector` (`self.Speed`))))
      (:`NewEnumerator2`
        (`self.K2_AddActorWorldOffset` (`KismetMathLibrary.MakeVector` 0.0 (`self.Speed`)))))
    (else
      (`KismetSystemLibrary.K2_PauseTimerHandle` (stale `self.StopHold` _returnvalue)))))

(fn `CheckFinish`
  (params (`Reverse?` :type Boolean))
  (returns (stop :type Boolean))
  (bind (_returnvalue_x _returnvalue_y _returnvalue_z) (`KismetMathLibrary.BreakVector` (`self.K2_GetActorLocation`)))
  (if (< (select `/Game/SoullessGames/Proto/Core/Enum/E_MovementsDirection` (`self.Movement Direction`) :`NewEnumerator0` _returnvalue_z :`NewEnumerator1` _returnvalue_x :`NewEnumerator2` _returnvalue_y) (`self.Valeur Min`))
    (return true)
    (else
      (return false))))

(fn `CheckSlide`
  (params (ValueToAdd :type "Float (double-precision)"))
  (returns (ReturnValue :type Boolean))
  (bind (_returnvalue_x _returnvalue_y _returnvalue_z) (`KismetMathLibrary.BreakVector` (`self.K2_GetActorLocation`)))
  (if (< ValueToAdd 0.0)
    _
    (elif (< (select `/Game/SoullessGames/Proto/Core/Enum/E_MovementsDirection` (`self.Movement Direction`) :`NewEnumerator0` _returnvalue_z :`NewEnumerator1` _returnvalue_x :`NewEnumerator2` _returnvalue_y) (`self.ValeurMax`))
      (return true)
      (else
        _)))
  (return false))

(fn `SetValeurMovement`
  (bind (_returnvalue_roll _returnvalue_pitch) (`KismetMathLibrary.BreakRotator` (`self.K2_GetActorRotation`)))
  (set `self.Valeur Min` _returnvalue_pitch)
  (set `self.ValeurMax` (+ (`self.Valeur Min`) (* 128.0 (`self.MovementPosible`)))))

(fn `UserConstructionScript`
  (`parent.UserConstructionScript`))