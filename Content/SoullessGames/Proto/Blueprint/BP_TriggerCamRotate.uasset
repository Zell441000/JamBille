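; Trigger volume actor that starts a camera rotation sequence when the player character (BP_Character) enters its box.
; On overlap it calls CallCamRotate on the game mode, activates every BP_ruines_2 in the level and removes the main UI.
; The overlap has no once-only guard.
; A delayed final score and end screen chain is present but unconnected, so it never runs.
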(event `self.Box.OnComponentBeginOverlap`
  (params (OverlappedComponent :type "PrimitiveComponent Object Reference") (OtherActor :type "Actor Object Reference") (OtherComp :type "PrimitiveComponent Object Reference") (OtherBodyIndex :type Integer) (bFromSweep :type Boolean) (SweepResult :type "HitResult Structure (by ref)"))
  (cast `/Game/SoullessGames/Proto/Player/BP_Character` OtherActor)
  (`/Game/SoullessGames/Proto/Player/BP_GameMode.CamRotate` (`/Game/SoullessGames/Proto/Core/BP_Library.GetMyGamemode`))
  (`|ExecutionSequence`
    (:`then_0`
      (bind _outactors (`GameplayStatics.GetAllActorsOfClass` "/Game/SoullessGames/Proto/Enviro/BP_ruines_2.BP_ruines_2_C"))
      (for _array_element _outactors
        (`/Game/SoullessGames/Proto/Enviro/BP_ruines_2.Activated` _array_element)))
    (:`then_1`
      (`Widget.RemoveFromParent` (`/Game/SoullessGames/Proto/Player/BP_GameMode.MainUi` (`/Game/SoullessGames/Proto/Core/BP_Library.GetMyGamemode`))))))

(fn `UserConstructionScript`)